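; Player actor for mouse-driven, grid-based board play that selects characters and orders them to move.
; BeginPlay shows the mouse and spawns a BP_Cursor3D, which Tick snaps to the grid cell under the cursor, oriented by the surface normal.
; Click selects or switches BP_BoardCharacterBase units, or sends the selected one to the snapped cell via AIMoveTo within a fixed range.
; MPC_Floor parameter updates exist but are unconnected.
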(event EventBeginPlay
  (bind _asplayer_controller (Utilities|Casting|CastToPlayerController (Pawn|GetController)))
  (bind _output_get (Variables|Default|SetContoller _asplayer_controller))
  (Variables|/Script/Engine.PlayerController|SetbShowMouseCursor _output_get true)
  (bind _returnvalue (Game|SpawnActorfromClass "/Game/Blueprints/BP_Cursor3D.BP_Cursor3D_C" (Transformation|GetActorTransform) "Undefined" 0 0))
  (Variables|Default|Set3DCursor _returnvalue))

(event Collision|EventActorBeginOverlap
  (params (OtherActor :type Actor%20Object%20Reference)))

(event EventTick
  (params (DeltaSeconds :type Float%20%28single-precision%29))
  (bind _contoller (Variables|Default|GetContoller))
  (bind _gridsize (Variables|Default|GetGridSize))
  (bind _hitresult (Game|Player|GetHitResultUnderCursorbyChannel _contoller "TraceTypeQuery1" true))
  (bind (_bblockinghit _binitialoverlap _time _distance _location _impactpoint _normal _impactnormal) (Collision|BreakHitResult _hitresult))
  (bind (_x _y _z) (Math|Vector|BreakVector _location))
  (Transformation|SetActorLocationAndRotation (Variables|Default|Get3DCursor) (* (Math|Vector|MakeVector (+ (Math|Conversions|ToFloat(Integer) (Math|Float|Floor (/ _x _gridsize))) 0.5) (+ (Math|Conversions|ToFloat(Integer) (Math|Float|Floor (/ _y _gridsize))) 0.5) _z) (Variables|Default|GetGridSize)) (Math|Rotator|MakeRotationfromAxes "0, 0, 0" _impactnormal "0, 0, 0")))

(event Input|ActionEvents|InputActionClick
  (params (Key :type Key%20Structure :default "None"))
  (bind _contoller (Variables|Default|GetContoller))
  (bind _contoller_2 (Variables|Default|GetContoller))
  (bind _gridsize (Variables|Default|GetGridSize))
  (bind _gridsize_2 (Variables|Default|GetGridSize))
  (bind _hitresult (Game|Player|GetHitResultUnderCursorbyChannel _contoller "TraceTypeQuery1" true))
  (bind _hitresult_2 (Game|Player|GetHitResultUnderCursorbyChannel _contoller_2 "TraceTypeQuery1" true))
  (bind _hitactor (Collision|BreakHitResult _hitresult))
  (bind (_bblockinghit _binitialoverlap _time _distance _location _impactpoint _normal _impactnormal) (Collision|BreakHitResult _hitresult_2))
  (bind (_x _y _z) (Math|Vector|BreakVector _location))
  (bind _returnvalue (/ _x _gridsize))
  (bind _returnvalue_2 (/ _y _gridsize))
  (bind _returnvalue_3 (Math|Float|Floor _returnvalue))
  (bind _returnvalue_4 (Math|Float|Floor _returnvalue_2))
  (bind _returnvalue_5 (Math|Conversions|ToFloat(Integer) _returnvalue_3))
  (bind _returnvalue_6 (Math|Conversions|ToFloat(Integer) _returnvalue_4))
  (bind _returnvalue_7 (+ _returnvalue_6 0.5))
  (bind _returnvalue_8 (+ _returnvalue_5 0.5))
  (bind _returnvalue_9 (Math|Vector|MakeVector _returnvalue_8 _returnvalue_7 _z))
  (bind _returnvalue_10 (* _returnvalue_9 _gridsize_2))
  (:Pressed
    (Utilities|IsValid (Variables|Default|GetCurrentlySelectedUnit)
      (:Is%20Valid
        (if (and (Actor|ActorHasTag _hitactor "Character") (Actor|ActorHasTag _hitactor "Character"))
          (Default|BeDeselected (Variables|Default|GetCurrentlySelectedUnit))
          (bind _asbp_board_character_base (Utilities|Casting|CastToBP_BoardCharacterBase _hitactor))
          (Default|BeSelected _asbp_board_character_base)
          (Variables|Default|SetCurrentlySelectedUnit _asbp_board_character_base)
          (elif (< (Math|Vector|Distance(Vector) _returnvalue_10 (Transformation|GetActorLocation (Variables|Default|GetCurrentlySelectedUnit))) 6e+02)
            (AI|AIMoveTo (Variables|Default|GetCurrentlySelectedUnit) _returnvalue_10 0 5.0 false))))
      (:Is%20Not%20Valid
        (bind _asbp_board_character_base_2 (Utilities|Casting|CastToBP_BoardCharacterBase _hitactor))
        (Default|BeSelected _asbp_board_character_base_2)
        (bind _output_get (Variables|Default|SetCurrentlySelectedUnit _asbp_board_character_base_2))))))

(fn ConstructionScript)